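; BP_Religion is an actor that represents a religion through a sprite and looping audio matching its dominant ritual type: Aggressive, Communal or Meditiative.
; BeginPlay starts the audio after a random delay of up to six seconds.
; Tick polls GetHighestRitualType and, on a change, stores the type, then swaps the sprite and restarts the matching sound.
; UpdateParticle only sets a second sprite's visibility from IsThePlayer; ShowAsThePlayer is empty.
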(event EventBeginPlay
  (Utilities|FlowControl|Delay (Math|Random|RandomFloatinRange 0.0 6.0))
  (Audio|Components|Audio|Play (Variables|Default|GetAudio) 0.0))

(event EventActorBeginOverlap
  (params (OtherActor :type Actor%20Object%20Reference)))

(event EventTick
  (params (DeltaSeconds :type Float%20%28single-precision%29))
  (bind _returnvalue (Class|Religion|GetHighestRitualType))
  (if (Utilities|Enum|NotEqual(Enum) (Variables|Default|GetType) _returnvalue)
    (Variables|Default|SetType _returnvalue)
    (Utilities|FlowControl|Sequence
      (:then_0
        (|UpdateSprite))
      (:then_1
        (|UpdateParticle))
      (:then_2
        (|UpdateSound)))))

(fn ConstructionScript)

(fn ShowasthePlayer)