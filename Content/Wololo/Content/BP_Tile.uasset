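; Map tile Blueprint that visualises the population and religious makeup of its area.
; Each tick, a dynamic material takes a normalised, share-weighted blend of religion colours, with emissive and opacity driven by population.
; Whenever population more than doubles since last growth, a spare mesh component becomes a building for the strongest religion's top ritual type, randomly placed and rotated.
; Cursor hover boosts the tile's glow.
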(event EventTick
  (params (DeltaSeconds :type Float%20%28single-precision%29))
  (bind _returnvalue (Class|Tile|GetPopulation))
  (Utilities|FlowControl|Sequence
    (:then_0
      (|SetColour))
    (:then_1
      (if (> _returnvalue (* (Variables|Default|GetLast%20Grown%20Population) 2))
        (bind (_empty_mesh_component _did_we_find_an_empty_mesh_component) (CallFunction|GetFirstEmptyMesh))
        (if _did_we_find_an_empty_mesh_component
          (Variables|Default|SetLast%20Grown%20Population _returnvalue)
          (Components|StaticMesh|SetStaticMesh _empty_mesh_component (Utilities|Select :Index (Class|Religion|GetHighestRitualType (Class|Tile|GetStrongestReligion)) :Aggressive "/Game/Wololo/Assets/Alter.Alter" :Communal "/Game/Wololo/Assets/church.church" :Meditiative "/Game/Wololo/Assets/hut.hut" :MAX 0))
          (Transformation|SetRelativeRotation _empty_mesh_component (Math|Random|RandomRotator false) false false)
          (Transformation|SetRelativeLocation _empty_mesh_component (* (Math|Random|RandomUnitVector) 5e+01) false false))))))

(event EventBeginPlay
  (Utilities|FlowControl|Sequence
    (:then_0
      (bind _returnvalue (Rendering|Material|CreateDynamicMaterialInstance (Variables|Default|GetTile) 0 (Rendering|Material|GetMaterial (Variables|Default|GetTile) 0) :!class /Script/Engine.PrimitiveComponent))
      (Variables|Default|SetMID _returnvalue))
    (:then_1
      (bind _output_get (Variables|Default|SetAll%20Empty%20Meshes (Actor|GetComponentsByClass "/Script/Engine.StaticMeshComponent")))
      (Utilities|Array|RemoveItem _output_get (Variables|Default|GetTile)))))

(event MouseInput|EventActorBeginCursorOver
  (Rendering|Material|SetScalarParameterValue (Variables|Default|GetMID) "ExtraEmissive" 2.0 :!class /Script/Engine.MaterialInstanceDynamic))

(event MouseInput|EventActorEndCursorOver
  (Rendering|Material|SetScalarParameterValue (Variables|Default|GetMID) "ExtraEmissive" 1.0 :!class /Script/Engine.MaterialInstanceDynamic))

(fn ConstructionScript)

(fn GetFirstEmptyMesh
  (bind _all_empty_meshes (Variables|Default|GetAll%20Empty%20Meshes))
  (if (> (Utilities|Array|Length _all_empty_meshes) 0)
    (bind _output_get (LocalVariables|SetReturn%20value (Utilities|Array|Get(acopy) _all_empty_meshes)))
    (Utilities|Array|RemoveIndex _all_empty_meshes)
    (return _output_get true)
    (else
      (return 0 false))))