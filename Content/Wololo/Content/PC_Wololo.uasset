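; Player controller for a tile-based religion game, handling camera control, tile selection and HUD creation.
; Scroll and right-mouse drag axes pan the Wololo pawn, scaled by orthographic width so speed follows the exponential, clamped zoom.
; Left click traces under the cursor on the Vehicle object type, passes the hit Tile to the HUD and overrides the audio listener.
; SpawnHud builds the HUD from the pawn's religion and a supplied ReligionManager.
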(event EventBeginPlay
  (Utilities|FlowControl|Sequence
    (:then_0
      (|SaveOurPawn))
    (:then_1
      (|SaveTileManager))))

(event Input|ActionEvents|InputActionSelectTileWithMouse
  (params (Key :type Key%20Structure :default "AnyKey"))
  (bind (_worldlocation _worlddirection) (Game|Player|ConvertMouseLocationToWorldSpace))
  (:Pressed
    (if (== Key "LeftMouseButton")
      (bind _outhit (Collision|LineTraceForObjects _worldlocation (+ _worldlocation (* _worlddirection 2e+03)) (Utilities|Array|MakeArray "ObjectTypeQuery5") false 0 "None"))
      (Utilities|IsValid (.HitActor (Collision|BreakHitResult _outhit))
        (:Is%20Valid
          (bind _astile (Utilities|Casting|CastToTile (.HitActor (Collision|BreakHitResult _outhit))))
          (Variables|/Game/Wololo/Content/BP_HUD.BP_HUD_C|SetTile (Variables|Default|GetHUD) _astile)
          (Class|PlayerController|SetAudioListenerOverride (Variables|Default|GetAudio%20Listener) "0, 0, 0" "0, 0, 0"))))))

(event Input|AxisEvents|InputAxisDragRight
  (params (AxisValue :type Float%20%28single-precision%29))
  (if (CallFunction|IsRightMouseButtonDown)
    (Default|AcceptScrollInput (Variables|Default|GetOur%20Wololo) (* "0.000000,1.000000, 0" (* AxisValue (Variables|Default|GetHeightModW))))))

(event Input|AxisEvents|InputAxisScrollRight
  (params (AxisValue :type Float%20%28single-precision%29))
  (Default|AcceptScrollInput (Variables|Default|GetOur%20Wololo) (* "0.000000,1.000000, 0" (* (Variables|Default|GetHeightModW) AxisValue))))

(event Input|AxisEvents|InputAxisScrollIn
  (params (AxisValue :type Float%20%28single-precision%29))
  (bind _our_wololo (Variables|Default|GetOur%20Wololo))
  (bind _camera (Variables|/Game/Wololo/Content/BP_WololoPawn.BP_WololoPawn_C|GetCamera _our_wololo))
  (Variables|/Script/Engine.CameraComponent|SetOrthoWidth _camera (Math|Float|Clamp(Float) (* (Math|Float|Power 1.001 AxisValue) (Variables|/Script/Engine.CameraComponent|GetOrthoWidth _camera)) 1.0 2.048e+04))
  (CallFunction|UpdateHeightMod))

(event Input|AxisEvents|InputAxisDragUp
  (params (AxisValue :type Float%20%28single-precision%29))
  (if (CallFunction|IsRightMouseButtonDown)
    (Default|AcceptScrollInput (Variables|Default|GetOur%20Wololo) (* "1.000000,0.000000, 0" (* AxisValue (Variables|Default|GetHeightModH))))))

(event Input|AxisEvents|InputAxisScrollUp
  (params (AxisValue :type Float%20%28single-precision%29))
  (Default|AcceptScrollInput (Variables|Default|GetOur%20Wololo) (* "1.000000,0.000000, 0" (* (Variables|Default|GetHeightModH) AxisValue))))

(fn ConstructionScript)

(fn IsRightMouseButtonDown
  (return (> (Class|PlayerController|GetInputKeyTimeDown "RightMouseButton") 0.0)))

(fn UpdateHeightMod
  (bind _our_wololo (Variables|Default|GetOur%20Wololo))
  (bind _camera (Variables|/Game/Wololo/Content/BP_WololoPawn.BP_WololoPawn_C|GetCamera _our_wololo))
  (bind _orthowidth (Variables|/Script/Engine.CameraComponent|GetOrthoWidth _camera))
  (Variables|Default|SetHeightModH (Math|Float|Max(Float) (/ (/ _orthowidth (Variables|/Script/Engine.CameraComponent|GetAspectRatio _camera)) 1024.0) 1.0))
  (Variables|Default|SetHeightModW (Math|Float|Max(Float) (/ _orthowidth 1024.0) 1.0))
  (return))

(fn SpawnHud
  (params (Religion%20Manager :type BP%20Religion%20Manager%20Object%20Reference))
  (bind _asbp_wololo_pawn (Utilities|Casting|CastToBP_WololoPawn (Pawn|GetControlledPawn)))
  (bind _returnvalue (UserInterface|CreateWidget "/Game/Wololo/Content/BP_HUD.BP_HUD_C"))
  (Variables|/Game/Wololo/Content/BP_HUD.BP_HUD_C|SetReligion _returnvalue (Variables|/Game/Wololo/Content/BP_WololoPawn.BP_WololoPawn_C|GetMy%20Religion _asbp_wololo_pawn))
  (UserInterface|Viewport|AddtoViewport _returnvalue 0)
  (bind _output_get (Variables|Default|SetHUD _returnvalue))
  (Variables|/Game/Wololo/Content/BP_HUD.BP_HUD_C|SetReligion%20Manager _output_get Religion%20Manager)
  (return _output_get))